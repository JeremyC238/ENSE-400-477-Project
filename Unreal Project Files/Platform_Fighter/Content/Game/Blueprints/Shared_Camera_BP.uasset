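; Shared camera actor that both local players view through, zooming with the distance between them.
; On BeginPlay it becomes both controllers' view target and stores the first two PlayerController actors as P1 and P2.
; A fast looping timer sets spring arm length to the distance between those controllers, clamped to min and max.
; Unconnected leftover graphs hold midpoint following, player clamping, player-count loading and alternative setups.
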(event Custom|UpdateCamera
  (Variables|/Script/Engine.SpringArmComponent|SetTargetArmLength (Variables|Default|GetSpringArm) (Math|Float|Clamp(Float) (Transformation|GetDistanceTo (Variables|Default|GetP1) (Variables|Default|GetP2)) (Variables|Default|GetMinArmLength) (Variables|Default|GetMaxArmLength))))

(event EventBeginPlay
  (Game|Player|SetViewTargetwithBlend (Game|GetPlayerController 1) self 0.0 "VTBlend_Linear" 0.0 false)
  (bind _outactors (Actor|GetAllActorsOfClass "/Script/Engine.PlayerController"))
  (Variables|Default|SetP1 (Utilities|Array|Get(acopy) _outactors))
  (Variables|Default|SetP2 (Utilities|Array|Get(acopy) _outactors 1))
  (Utilities|Time|SetTimerbyFunctionName 0 "UpdateCamera" 0.001 true))

(event EventTick
  (params (DeltaSeconds :type Float%20%28single-precision%29)))

(fn ConstructionScript)