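; One-way stage platform that the two local players can jump up through and land on.
; The Cube ignores the Pawn channel by default, and the Box overlap switches it to Block for player 0 or 1.
; Blocking is immediate if the player's mesh is above the Cube, otherwise delayed briefly to let them pass.
; Either player ending overlap restores Ignore, as collision is toggled per channel rather than per player.
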(event OnComponentBeginOverlap(Box)
  (params (OverlappedComponent :type Primitive%20Component%20Object%20Reference) (OtherActor :type Actor%20Object%20Reference) (OtherComp :type Primitive%20Component%20Object%20Reference) (OtherBodyIndex :type Integer) (bFromSweep :type Boolean) (SweepResult :type Hit%20Result%20Structure%20%28by%20ref%29))
  (bind _returnvalue (Game|GetPlayerCharacter 0))
  (bind _returnvalue_2 (Game|GetPlayerCharacter 1))
  (bind _cube (Variables|Default|GetCube))
  (bind _returnvalue_3 (Transformation|GetWorldLocation _cube))
  (bind _z (Math|Vector|BreakVector _returnvalue_3))
  ;[1 1 1] pushes the player one way or the other through the platform based on the height or z axis of the character / update the platform to block the player from falling through
  (if (== OtherActor _returnvalue)
    (if (> (.Z (Math|Vector|BreakVector (Transformation|GetWorldLocation (Variables|/Script/Engine.Character|GetMesh _returnvalue)))) _z)
      _
      (else
        (Utilities|FlowControl|Delay 0.2 :!label _label)))
    (Collision|SetCollisionResponsetoChannel (Variables|Default|GetCube) "ECC_Pawn" "ECR_Block" :!label _label_2)
    (elif (== OtherActor _returnvalue_2)
      (if (> (.Z (Math|Vector|BreakVector (Transformation|GetWorldLocation (Variables|/Script/Engine.Character|GetMesh _returnvalue_2)))) _z)
        (goto _label_2)
        (else
          (goto _label))))))

(event OnComponentEndOverlap(Box)
  (params (OverlappedComponent :type Primitive%20Component%20Object%20Reference) (OtherActor :type Actor%20Object%20Reference) (OtherComp :type Primitive%20Component%20Object%20Reference) (OtherBodyIndex :type Integer))
  ;[1 1 1] once the overlap with the platform ends the player is able to jump through the platform again
  (if (== OtherActor (Game|GetPlayerCharacter 0))
    (Collision|SetCollisionResponsetoChannel (Variables|Default|GetCube) "ECC_Pawn" "ECR_Ignore" :!label _label)
    (elif (== OtherActor (Game|GetPlayerCharacter 1))
      (goto _label))))

(event EventBeginPlay
  ;[1 1 1] allows the player to jump through the platform on startup
  (Collision|SetCollisionResponsetoChannel (Variables|Default|GetCube) "ECC_Pawn" "ECR_Ignore"))

(fn ConstructionScript)